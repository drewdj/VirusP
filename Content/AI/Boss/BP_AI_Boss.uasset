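; Boss AI character that sets its base damage and experience on BeginPlay, on top of inherited parent logic.
; When its Health fires OnDeath, it deactivates boss combat on its AI controller, stops boss music and plays a damage sound.
; After a short delay it unpauses the player's base music, clears the sword mesh and spawns a weapon actor at the sword's location.
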(event OnDeath(Health)
  (bind _sword (Variables|Default|GetSword))
  (bind _returnvalue (Transformation|GetWorldTransform _sword))
  (bind _asbp_ai_controller_generic_boss (Utilities|Casting|CastToBP_AI_Controller_Generic_Boss (Pawn|GetController)))
  (Default|DeactivateBossCombat _asbp_ai_controller_generic_boss)
  (bind _bossmusic (Variables|Default|GetBossMusic)
    (:then
      (Audio|Components|Audio|Stop _bossmusic))
    (:else
      _))
  (Audio|PlaySoundatLocation "/Game/Audio/enemy/damage_Cue.damage_Cue" (Transformation|GetActorLocation) "0, 0, 0" 1.0 0.3 0.0 0 0 0 0)
  (Utilities|FlowControl|Delay 2.0)
  (Class|AudioComponent|SetPaused (Variables|/Game/ThirdPerson/Blueprints/BP_ThirdPersonCharacter.BP_ThirdPersonCharacter_C|GetBaseMusic (Variables|Default|GetPlayerCharacter)) false)
  (Components|StaticMesh|SetStaticMesh (Variables|Default|GetSword) 0)
  (Game|SpawnActorfromClass :Class "/Game/EquipmentSystem/BP_Weapon.BP_Weapon_C" :SpawnTransform (Math|Transform|MakeTransform (.location _returnvalue) "0, 0, 0" (.scale _returnvalue)) :CollisionHandlingOverride "Undefined" :Instigator 0)
  (Development|PrintString "Muerto2"))

(event Custom|Dead
  (Development|PrintString "Muerto"))

(event EventBeginPlay
  (|CallParentFunction)
  (Variables|Default|SetBase%20Damage 1e+01)
  (Variables|Default|SetExperience 5e+02))

(event Collision|EventActorBeginOverlap
  (params (OtherActor :type Actor%20Object%20Reference)))

(event EventTick
  (params (DeltaSeconds :type Float%20%28single-precision%29))
  (|CallParentFunction DeltaSeconds))

(fn ConstructionScript
  (|CallParentFunction))