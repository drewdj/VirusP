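; Base melee enemy character with health, XP reward on death, world-space health, investigate and soft-lock widgets, and material-driven alert states.
; Behavior tree attacks run a buffered montage combo, dealing damage through weapon overlap or sphere trace while Tick turns it toward the target.
; A timed Rage state notifies the AI controller and lets weapon hits damage fellow AI.
; Damage triggers knockback and slowed-time stagger; death briefly slows global time.
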(event OnDeath(Health)
  (Utilities|Time|SetGlobalTimeDilation 0.3)
  (Class|LevelComponent|AddExperience (Variables|/Script/VirusP.VirusPCharacter|GetLevelComponent (Variables|Default|GetPlayerCharacter)) (Variables|Default|GetExperience))
  (CallFunction|RedAlertOff)
  (bind _asbp_ai_controller_generic (Utilities|Casting|CastToBP_AI_Controller_Generic (Pawn|GetController))
    (:then
      (Default|Killed _asbp_ai_controller_generic))
    (:CastFailed
      _))
  (Rendering|SetVisibility (Variables|Default|GetHealthBarWidget) false false)
  (Collision|SetCollisionEnabled (Variables|Collision|GetCapsuleComponent) "NoCollision")
  ;[1 1 1] Cambiar a  solo si he matado al que tengo lockeado
  (Default|DisableTargetLock (Variables|Default|GetPlayerCharacter))
  (Utilities|FlowControl|Delay 0.3)
  (Utilities|Time|SetGlobalTimeDilation 1.0)
  (Utilities|FlowControl|Delay 1.0)
  (bind _asbp_ai_boss (Utilities|Casting|CastToBP_AI_Boss self))
  (Default|Dead _asbp_ai_boss))

(event OnComponentBeginOverlap(WeaponHitbox)
  (params (OverlappedComponent :type Primitive%20Component%20Object%20Reference) (OtherActor :type Actor%20Object%20Reference) (OtherComp :type Primitive%20Component%20Object%20Reference) (OtherBodyIndex :type Integer) (bFromSweep :type Boolean) (SweepResult :type Hit%20Result%20Structure%20%28by%20ref%29))
  (if (!= OtherActor self)
    (if (Variables|Default|GetRage)
      _
      (else
        (Utilities|Casting|CastToBP_AI OtherActor
          (:CastFailed
            _))))
    (Class|AISenseDamage|ReportDamageEvent OtherActor self 0.0 "0, 0, 0" "0, 0, 0" "None")
    (Game|Damage|ApplyDamage OtherActor (+ (Variables|Default|GetBase%20Damage) 1e+01) 0 0)))

(event Custom|SwordAttack
  ;[0.06354 0.06354 0.06354] ComboSystem
  ;;[0.06354 0.06354 0.06354] SwordAttack
  (if (Variables|Default|GetStagger)
    (Utilities|FlowControl|Delay 1.0)
    (Variables|Default|SetCustomTimeDilation 1.0))
  (if (Variables|Default|GetisAttacking?)
    (Variables|Default|SetsaveAttack true)
    (else
      (Variables|Default|SetisAttacking? true)
      (switch int (Variables|Default|GetattackIndex)
        (:0
          (CallFunction|Attack1))
        (:1
          (CallFunction|Attack2))
        (:2
          (CallFunction|Attack4))))))

(event Custom|SwordAttackCombo
  ;[0.06354 0.06354 0.06354] ComboSystem
  ;;[0.06354 0.06354 0.06354] ComboContinue
  (if (Variables|Default|GetsaveAttack)
    (Variables|Default|SetsaveAttack false)
    (switch int (Variables|Default|GetattackIndex)
      (:0
        (CallFunction|Attack1))
      (:1
        (CallFunction|Attack2))
      (:2
        (CallFunction|Attack4)))
    (else
      (CallFunction|StopCombo))))

(event Custom|Sword%20Attack%20Combo%20Call%20From%20BT
  ;[0.06354 0.06354 0.06354] ComboSystem
  ;;[0.06354 0.06354 0.06354] AttackInput
  (if (Variables|Default|GetcanAttack?)
    (CallFunction|SwordAttack)))

(event Custom|SetEnemy
  (Variables|Default|SetRage true)
  (CallFunction|Rageon)
  (Utilities|FlowControl|Delay 15.0)
  (Variables|Default|SetRage false)
  (CallFunction|RageOff))

(event Custom|RedAlertOn
  (bind _mesh (Variables|Character|GetMesh))
  (bind _enemymaterial (Variables|Default|GetEnemyMaterial))
  (Rendering|Material|SetScalarParameterValue _enemymaterial "RedAlert" 1.0 :!class /Script/Engine.MaterialInstanceDynamic)
  (Rendering|Material|SetMaterial _mesh 0 _enemymaterial)
  (Rendering|Material|SetMaterial _mesh 1 _enemymaterial)
  (Development|PrintString "RedAler"))

(event Custom|RageOff
  (bind _mesh (Variables|Character|GetMesh))
  (bind _enemymaterial (Variables|Default|GetEnemyMaterial))
  (Rendering|Material|SetScalarParameterValue _enemymaterial "Rage" 0.0 :!class /Script/Engine.MaterialInstanceDynamic)
  (Rendering|Material|SetMaterial _mesh 0 _enemymaterial)
  (Rendering|Material|SetMaterial _mesh 1 _enemymaterial)
  (bind _asbp_ai_controller_generic (Utilities|Casting|CastToBP_AI_Controller_Generic (Pawn|GetController)))
  (Default|Rage _asbp_ai_controller_generic)
  (Development|PrintString "Rage"))

(event Custom|RedAlertOff
  (bind _mesh (Variables|Character|GetMesh))
  (bind _enemymaterial (Variables|Default|GetEnemyMaterial))
  (Rendering|Material|SetScalarParameterValue _enemymaterial "RedAlert" 0.0 :!class /Script/Engine.MaterialInstanceDynamic)
  (Rendering|Material|SetMaterial _mesh 0 _enemymaterial)
  (Rendering|Material|SetMaterial _mesh 1 _enemymaterial))

(event Custom|DisableSoftlockIcon
  (Rendering|SetVisibility (Variables|Default|GetSoftlockWidget) false false))

(event Custom|StopCombo
  ;[0.06354 0.06354 0.06354] ComboSystem
  ;;[0.06354 0.06354 0.06354] StopCombo/Attack
  (Utilities|FlowControl|Delay 1.0)
  (Variables|Default|SetisAttacking? false)
  (Variables|Default|SetattackIndex 0))

(event Custom|RageOn
  (bind _mesh (Variables|Character|GetMesh))
  (bind _enemymaterial (Variables|Default|GetEnemyMaterial))
  (Rendering|Material|SetScalarParameterValue _enemymaterial "Rage" 1.0 :!class /Script/Engine.MaterialInstanceDynamic)
  (Rendering|Material|SetMaterial _mesh 0 _enemymaterial)
  (Rendering|Material|SetMaterial _mesh 1 _enemymaterial)
  (bind _asbp_ai_controller_generic (Utilities|Casting|CastToBP_AI_Controller_Generic (Pawn|GetController)))
  (Default|Rage _asbp_ai_controller_generic)
  (Development|PrintString "Rage"))

(event Custom|Toggle%20Investigation%20Icon
  (bind _investigatewidget (Variables|Default|GetInvestigateWidget))
  (Utilities|FlowControl|FlipFlop
    (:A
      (Rendering|SetVisibility _investigatewidget true false))
    (:B
      (Rendering|SetVisibility _investigatewidget false false))))

(event Custom|EnableSoftlockIcon
  (Rendering|SetVisibility (Variables|Default|GetSoftlockWidget) true false))

(event Custom|Attack4
  ;[0.06354 0.06354 0.06354] ComboSystem
  ;;[0.06354 0.06354 0.06354] Attack4
  (Utilities|FlowControl|DoOnce false :!label _label
    (:Completed
      (Utilities|FlowControl|Delay 0.1)
      (Animation|Montage|PlayMontage (Variables|Character|GetMesh) "/Game/Characters/VirusP_Character/Animations/OneHandedSword/Attack3_Montage.Attack3_Montage" (Variables|Default|GetAttackAnimationSpeed)
        (:then
          (Variables|Default|SetattackIndex 4)
          (goto _label Reset))))))

(event Custom|Attack%201
  ;[0.06354 0.06354 0.06354] ComboSystem
  ;;[0.06354 0.06354 0.06354] Attack1
  (Utilities|FlowControl|DoOnce false :!label _label
    (:Completed
      (Utilities|FlowControl|Delay 0.1)
      (Animation|Montage|PlayMontage (Variables|Character|GetMesh) "/Game/Characters/VirusP_Character/Animations/OneHandedSword/Attack1Short_Montage.Attack1Short_Montage" (Variables|Default|GetAttackAnimationSpeed)
        (:then
          (Variables|Default|SetattackIndex 1)
          (goto _label Reset))))))

(event Custom|Sphere%20Trace
  (bind _sphere_trace1 (Variables|Default|GetSphere%20Trace1))
  (bind _returnvalue (Transformation|GetWorldLocation _sphere_trace1))
  ;[0.06354 0.06354 0.06354] Sphere Trace(stab and kick)
  (bind (_outhit _returnvalue_2) (Collision|SphereTraceByChannel _returnvalue _returnvalue 25.0 "TraceTypeQuery1" false 0 "ForDuration"))
  (if _returnvalue_2
    (if (Actor|ActorHasTag (.HitActor (Collision|BreakHitResult _outhit)) "Damageable")
      (Class|AISenseDamage|ReportDamageEvent (.HitActor (Collision|BreakHitResult _outhit)) self 0.0 (.Location (Collision|BreakHitResult _outhit)) "0, 0, 0" "None")
      (Game|Damage|ApplyDamage (.HitActor (Collision|BreakHitResult _outhit)) (Variables|Default|GetBase%20Damage) 0 0))))

(event Custom|Attack2
  ;[0.06354 0.06354 0.06354] ComboSystem
  ;;[0.06354 0.06354 0.06354] Attack3
  (Utilities|FlowControl|DoOnce false :!label _label
    (:Completed
      (Utilities|FlowControl|Delay 0.1)
      (Animation|Montage|PlayMontage (Variables|Character|GetMesh) "/Game/Characters/VirusP_Character/Animations/OneHandedSword/Attack2_Montage.Attack2_Montage" (Variables|Default|GetAttackAnimationSpeed)
        (:then
          (Variables|Default|SetattackIndex 2)
          (goto _label Reset))))))

(event Custom|StopSwordCollision
  (Collision|SetCollisionEnabled (Variables|Default|GetWeaponHitbox) "NoCollision"))

(event Custom|Attack3
  ;[0.06354 0.06354 0.06354] ComboSystem
  ;;[0.06354 0.06354 0.06354] Attack3
  (Utilities|FlowControl|DoOnce false :!label _label
    (:Completed
      (Utilities|FlowControl|Delay 0.1)
      (Animation|Montage|PlayMontage (Variables|Character|GetMesh) "/Game/Characters/VirusP_Character/Animations/OneHandedSword/Kick_Montage.Kick_Montage" (Variables|Default|GetAttackAnimationSpeed)
        (:then
          (Variables|Default|SetattackIndex 3)
          (goto _label Reset))))))

(event Custom|StartSwordCollision
  (Collision|SetCollisionEnabled (Variables|Default|GetWeaponHitbox) "QueryAndPhysics"))

(event EventBeginPlay
  (bind _asbp_third_person_character (Utilities|Casting|CastToBP_ThirdPersonCharacter (Game|GetPlayerCharacter 0)))
  (Variables|Default|SetPlayerCharacter _asbp_third_person_character)
  (bind _returnvalue (Rendering|Material|CreateDynamicMaterialInstance "/Game/Materials/Enemy.Enemy" "None" "None" :!class /Script/Engine.KismetMaterialLibrary))
  (Variables|Default|SetEnemyMaterial _returnvalue))

(event Game|Damage|EventAnyDamage
  (params (Damage :type Float%20%28single-precision%29) (DamageType :type Damage%20Type%20Object%20Reference) (InstigatedBy :type Controller%20Object%20Reference) (DamageCauser :type Actor%20Object%20Reference))
  (Animation|PlayAnimMontage (Utilities|Array|Get(acopy) (Variables|Default|GetHitAnims) (Math|Random|RandomIntegerinRange 0 (- (Utilities|Array|Length (Variables|Default|GetHitAnims)) 1))) 1.0 "None")
  (CallFunction|StopCombo)
  (Character|LaunchCharacter (* (Math|Vector|GetForwardVector (Transformation|GetActorRotation (Variables|Default|GetPlayerCharacter))) 7e+02) false false)
  (Variables|Default|SetStagger true)
  (Variables|Default|SetCustomTimeDilation 0.5))

(event EventTick
  (params (DeltaSeconds :type Float%20%28single-precision%29))
  (bind _healthbarwidget (Variables|Default|GetHealthBarWidget))
  (bind _health (Variables|Default|GetHealth))
  (bind _aswbp_health_bar (Utilities|Casting|CastToWBP_HealthBar (UserInterface|GetWidget (Variables|Default|GetHealthBarWidget))))
  (Progress|SetPercent (Variables|/Game/Blueprints/Widgets/WBP_HealthBar.WBP_HealthBar_C|GetHealthBar _aswbp_health_bar) (/ (Variables|/Script/VirusP.HealthComponent|GetHealth _health) (Variables|/Script/VirusP.HealthComponent|GetDefaultHealth _health)))
  (Transformation|SetWorldRotation _healthbarwidget (Math|Rotator|FindLookatRotation (Transformation|GetWorldLocation _healthbarwidget) (Transformation|GetWorldLocation (Variables|/Script/Engine.PlayerCameraManager|GetTransformComponent (Game|GetPlayerCameraManager 0)))) false false)
  (bind _asbp_ai_controller_generic (Utilities|Casting|CastToBP_AI_Controller_Generic (Pawn|GetController)))
  (bind _attack_target (Variables|/Game/AI/BP_AI_Controller_Generic.BP_AI_Controller_Generic_C|GetAttack%20Target _asbp_ai_controller_generic)
    (:then
      (if (Variables|Default|GetisAttacking?)
        (Transformation|SetActorRotation (Math|Interpolation|RInterpTo (Transformation|GetActorRotation) (Math|Rotator|MakeRotator 0.0 0.0 (.yaw (Math|Rotator|FindLookatRotation (Transformation|GetActorLocation) (Transformation|GetActorLocation _attack_target)))) DeltaSeconds 1e+01))))
    (:else)))

(fn ConstructionScript)

(fn Attack
  (CallFunction|SwordAttackComboCallfromBT)
  (return 0.4))