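; Attack component for the third-person character that runs a four-step sword and kick montage combo.
; Input during an attack is buffered, and SwordAttackCombo either advances the combo index or resets it.
; A new combo launches the character toward the soft-locked enemy, and Tick turns it to face that target while attacking.
; Damage comes from a toggled weapon hitbox, with once-per-swing filtering and combo bonuses, or a sphere trace for stab and kick.
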(event Custom|SwordAttack
  ;[0.06354 0.06354 0.06354] ComboSystem
  ;;[0.06354 0.06354 0.06354] SwordAttack
  (if (Variables|Default|GetisAttacking?)
    (Variables|Default|SetsaveAttack true)
    (else
      (Variables|Default|SetisAttacking? true)
      (CallFunction|Dash)
      (switch int (Variables|Default|GetattackIndex)
        (:0
          (CallFunction|Attack1))
        (:1
          (CallFunction|Attack2))
        (:2
          (CallFunction|Attack3))
        (:3
          (CallFunction|Attack4))))))

(event Custom|SwordAttackCombo
  ;[0.06354 0.06354 0.06354] ComboSystem
  ;;[0.06354 0.06354 0.06354] ComboContinue
  (if (Variables|Default|GetsaveAttack)
    (Variables|Default|SetsaveAttack false)
    (switch int (Variables|Default|GetattackIndex)
      (:0
        (CallFunction|Attack1))
      (:1
        (CallFunction|Attack2))
      (:2
        (CallFunction|Attack3))
      (:3
        (CallFunction|Attack4)))
    (else
      (CallFunction|StopCombo))))

(event Custom|DealDamage
  (params (DamagedActor :type Actor%20Object%20Reference))
  (bind _damagedactors (Variables|Default|GetDamagedActors))
  (if (not (Utilities|Set|Contains _damagedactors DamagedActor))
    (Utilities|Set|Add _damagedactors DamagedActor)
    (Development|PrintString "DAMAGED")
    (Class|AISenseDamage|ReportDamageEvent DamagedActor (Variables|Default|GetCharacterBP) 0.0 "0, 0, 0" "0, 0, 0" "None")
    (switch int (Variables|Default|GetattackIndex)
      (:Default
        _)
      (:0
        (Variables|Default|SetComboDamage 0.0))
      (:1
        (Variables|Default|SetComboDamage 5.0))
      (:2
        (Variables|Default|SetComboDamage 1e+01))
      (:3
        (Variables|Default|SetComboDamage 2e+01)))
    (Game|Damage|ApplyDamage DamagedActor (+ (Variables|/Game/ThirdPerson/Blueprints/BP_ThirdPersonCharacter.BP_ThirdPersonCharacter_C|GetTempDamage (Variables|Default|GetCharacterBP)) (Variables|Default|GetComboDamage)) 0 0)))

(event Custom|StopCombo
  ;[0.06354 0.06354 0.06354] ComboSystem
  ;;[0.06354 0.06354 0.06354] StopCombo/Attack
  (Variables|Default|SetisAttacking? false)
  (Variables|Default|SetattackIndex 0))

(event Custom|Attack4
  ;[0.06354 0.06354 0.06354] ComboSystem
  ;;[0.06354 0.06354 0.06354] Attack4
  (Utilities|FlowControl|DoOnce false :!label _label
    (:Completed
      (Utilities|FlowControl|Delay 0.1)
      (Animation|Montage|PlayMontage (Variables|Default|GetcharacterMesh) "/Game/Characters/VirusP_Character/Animations/OneHandedSword/Attack3_Montage.Attack3_Montage"
        (:then
          (Variables|Default|SetattackIndex 4)
          (goto _label Reset))))))

(event Custom|Attack%201
  ;[0.06354 0.06354 0.06354] ComboSystem
  ;;[0.06354 0.06354 0.06354] Attack1
  (Utilities|FlowControl|DoOnce false :!label _label
    (:Completed
      (Utilities|FlowControl|Delay 0.1)
      (Animation|Montage|PlayMontage (Variables|Default|GetcharacterMesh) "/Game/Characters/VirusP_Character/Animations/OneHandedSword/Attack1Short_Montage.Attack1Short_Montage"
        (:then
          (Variables|Default|SetattackIndex 1)
          (goto _label Reset))))))

(event Custom|Sphere%20Trace
  (bind _characterbp (Variables|Default|GetCharacterBP))
  (bind _sphere_trace (Variables|/Game/ThirdPerson/Blueprints/BP_ThirdPersonCharacter.BP_ThirdPersonCharacter_C|GetSphere%20Trace _characterbp))
  (bind _returnvalue (Transformation|GetWorldLocation _sphere_trace))
  ;[0.06354 0.06354 0.06354] Sphere Trace(stab and kick)
  (bind (_outhit _returnvalue_2) (Collision|SphereTraceByChannel _returnvalue _returnvalue 25.0 "TraceTypeQuery1" false 0 "ForDuration"))
  (if _returnvalue_2
    (if (Actor|ActorHasTag (.HitActor (Collision|BreakHitResult _outhit)) "Damageable")
      (Class|AISenseDamage|ReportDamageEvent (.HitActor (Collision|BreakHitResult _outhit)) (Variables|Default|GetCharacterBP) 0.0 (.Location (Collision|BreakHitResult _outhit)) "0, 0, 0" "None")
      (Game|Damage|ApplyDamage (.HitActor (Collision|BreakHitResult _outhit)) (Variables|/Game/ThirdPerson/Blueprints/BP_ThirdPersonCharacter.BP_ThirdPersonCharacter_C|GetTempDamage (Variables|Default|GetCharacterBP)) 0 0))))

(event Custom|Attack2
  ;[0.06354 0.06354 0.06354] ComboSystem
  ;;[0.06354 0.06354 0.06354] Attack3
  (Utilities|FlowControl|DoOnce false :!label _label
    (:Completed
      (Utilities|FlowControl|Delay 0.1)
      (Animation|Montage|PlayMontage (Variables|Default|GetcharacterMesh) "/Game/Characters/VirusP_Character/Animations/OneHandedSword/Attack2_Montage.Attack2_Montage"
        (:then
          (Variables|Default|SetattackIndex 2)
          (goto _label Reset))))))

(event Custom|StopSwordCollision
  (Collision|SetCollisionEnabled (Variables|/Game/ThirdPerson/Blueprints/BP_ThirdPersonCharacter.BP_ThirdPersonCharacter_C|GetWeaponHitbox (Variables|Default|GetCharacterBP)) "NoCollision")
  (Utilities|Set|Clear (Variables|Default|GetDamagedActors)))

(event Custom|Attack3
  ;[0.06354 0.06354 0.06354] ComboSystem
  ;;[0.06354 0.06354 0.06354] Attack3
  (Utilities|FlowControl|DoOnce false :!label _label
    (:Completed
      (Utilities|FlowControl|Delay 0.1)
      (Animation|Montage|PlayMontage (Variables|Default|GetcharacterMesh) "/Game/Characters/VirusP_Character/Animations/OneHandedSword/Kick_Montage.Kick_Montage"
        (:then
          (Variables|Default|SetattackIndex 3)
          (goto _label Reset))))))

(event Custom|StartSwordCollision
  (bind _characterbp (Variables|Default|GetCharacterBP))
  (bind _weaponhitbox (Variables|/Game/ThirdPerson/Blueprints/BP_ThirdPersonCharacter.BP_ThirdPersonCharacter_C|GetWeaponHitbox _characterbp))
  (Collision|SetCollisionEnabled _weaponhitbox "QueryAndPhysics")
  (Collision|SetCollisionResponsetoAllChannels _weaponhitbox "ECR_Overlap"))

(event EventTick
  (params (DeltaSeconds :type Float%20%28single-precision%29))
  (bind _characterbp (Variables|Default|GetCharacterBP))
  (if (Variables|Default|GetisAttacking?)
    (bind _softlockedenemy (Variables|/Game/Blueprints/BPC_TargetingSystemComponent.BPC_TargetingSystemComponent_C|GetSoftLockedEnemy (Variables|/Game/ThirdPerson/Blueprints/BP_ThirdPersonCharacter.BP_ThirdPersonCharacter_C|GetBPC_TargetingSystemComponent _characterbp))
      (:then
        (Transformation|SetActorRotation _characterbp (Math|Interpolation|RInterpTo (Transformation|GetActorRotation _characterbp) (Math|Rotator|MakeRotator 0.0 0.0 (.yaw (Math|Rotator|FindLookatRotation (Transformation|GetActorLocation _characterbp) (Transformation|GetActorLocation _softlockedenemy)))) DeltaSeconds 1e+01)))
      (:else))))

(event EventBeginPlay
  (bind _asbp_third_person_character (Utilities|Casting|CastToBP_ThirdPersonCharacter (Components|GetOwner)))
  (Variables|Default|SetCharacterBP _asbp_third_person_character)
  (Variables|Default|SetcharacterMesh (Variables|/Script/Engine.Character|GetMesh _asbp_third_person_character)))

(event Input|ActionEvents|InputActionAttack
  (params (Key :type Key%20Structure :default "None"))
  ;[0.06354 0.06354 0.06354] ComboSystem
  ;;[0.06354 0.06354 0.06354] AttackInput
  (:Pressed
    (if (Variables|Default|GetArmed?)
      (if (Variables|Default|GetcanAttack?)
        (CallFunction|SwordAttack)))))

(fn Dash
  (bind _characterbp (Variables|Default|GetCharacterBP))
  (bind _softlockedenemy (Variables|/Game/Blueprints/BPC_TargetingSystemComponent.BPC_TargetingSystemComponent_C|GetSoftLockedEnemy (Variables|/Game/ThirdPerson/Blueprints/BP_ThirdPersonCharacter.BP_ThirdPersonCharacter_C|GetBPC_TargetingSystemComponent _characterbp))
    (:then
      (if (> (Transformation|GetDistanceTo _characterbp _softlockedenemy) 1.0)
        (Character|LaunchCharacter _characterbp (* (Math|Vector|GetForwardVector (Math|Rotator|FindLookatRotation (Transformation|GetActorLocation _characterbp) (Transformation|GetActorLocation _softlockedenemy))) 1e+03) true true)))
    (:else)))