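; BP_TextTutorial is a trigger actor that shows a one-time tutorial popup when the third-person character enters its box.
; The first overlap creates a WBP_TextTutorial widget and fills it with the actor's Text variable, also printed as a debug string.
; It then switches input to Game and UI, shows the mouse cursor and pauses the game, with no unpause logic in this Blueprint.
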(event OnComponentBeginOverlap(Box)
  (params (OverlappedComponent :type Primitive%20Component%20Object%20Reference) (OtherActor :type Actor%20Object%20Reference) (OtherComp :type Primitive%20Component%20Object%20Reference) (OtherBodyIndex :type Integer) (bFromSweep :type Boolean) (SweepResult :type Hit%20Result%20Structure%20%28by%20ref%29))
  (bind _returnvalue (Game|GetPlayerController 0))
  (bind _text (Variables|Default|GetText))
  ;[1 1 1] Tutorial UI
  (Utilities|Casting|CastToBP_ThirdPersonCharacter OtherActor)
  (Utilities|FlowControl|DoOnce false
    (:Completed
      (Development|PrintString _text)
      (bind _returnvalue_2 (UserInterface|CreateWidget "/Game/Maps/WBP_TextTutorial.WBP_TextTutorial_C"))
      (bind _output_get (Variables|Default|SetUI _returnvalue_2))
      (UserInterface|Viewport|AddtoViewport _output_get 0)
      (Rendering|Components|TextRender|SetText (Variables|/Game/Maps/WBP_TextTutorial.WBP_TextTutorial_C|GetText _output_get) (Utilities|Text|ToText(String) _text))
      (Input|SetInputModeGameandUI _returnvalue 0 "DoNotLock" true)
      (Variables|/Script/Engine.PlayerController|SetbShowMouseCursor _returnvalue true)
      (Game|SetGamePaused true))))

(fn ConstructionScript)