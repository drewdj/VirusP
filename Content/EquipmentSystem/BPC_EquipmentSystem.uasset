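; Player equipment component that holds the item inventory and toggles the equipment menu for the third-person character.
; Interact adds the externally set PickupItem to WeaponSlots, and AddWeapon looks up its data table type to auto-equip melee, bow, shield or heal items into empty slots.
; The menu blocks attacks and movement and nearly freezes time through global dilation.
; An old camera sphere-trace pickup remains unconnected, and H prints the inventory for debugging.
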(event EventBeginPlay
  ;[1 1 1] Set variables
  (bind _asbp_third_person_character (Utilities|Casting|CastToBP_ThirdPersonCharacter (Components|GetOwner)))
  (Variables|Default|SetAs%20BP%20Third%20Person%20Character _asbp_third_person_character)
  (Variables|Default|SetFollow%20Camera (Variables|/Script/VirusP.VirusPCharacter|GetFollowCamera _asbp_third_person_character))
  (Variables|Default|SetBPC%20Attack%20System%20Component (Variables|/Game/ThirdPerson/Blueprints/BP_ThirdPersonCharacter.BP_ThirdPersonCharacter_C|GetBPC_AttackSystemComponent _asbp_third_person_character)))

(event Input|ActionEvents|InputActionInteract
  (params (Key :type Key%20Structure))
  (:Pressed
    (bind _pickupitem (Variables|Default|GetPickupItem)
      (:then
        (CallFunction|AddWeapon (Variables|/Game/EquipmentSystem/BP_Weapon.BP_Weapon_C|GetItemData _pickupitem))
        (Actor|DestroyActor _pickupitem))
      (:else))))

(event Input|ActionEvents|InputActionEquipmentMenu
  (params (Key :type Key%20Structure))
  (bind _returnvalue (Game|GetPlayerController 0))
  (bind _bpc_attack_system_component (Variables|Default|GetBPC%20Attack%20System%20Component))
  ;[1 1 1] Equipment menu panel
  (:Pressed
    (if (not (Variables|Default|GetisPanelOpened))
      (Variables|/Game/Blueprints/BPC_AttackSystemComponent.BPC_AttackSystemComponent_C|SetcanAttack? _bpc_attack_system_component false)
      (Variables|Default|SetisPanelOpened true)
      (bind _returnvalue_2 (UserInterface|CreateWidget "/Game/Blueprints/Widgets/WBP_Equipment.WBP_Equipment_C"))
      (bind _output_get (Variables|Default|SetEquipmentWidget _returnvalue_2))
      (UserInterface|Viewport|AddtoViewport _output_get 0)
      (Variables|/Script/Engine.PlayerController|SetbShowMouseCursor _returnvalue true)
      (Input|SetInputModeGameandUI _returnvalue (Variables|Default|GetEquipmentWidget) "DoNotLock" true)
      (Pawn|Components|CharacterMovement|SetMovementMode (Variables|/Script/Engine.Character|GetCharacterMovement (Variables|Default|GetAs%20BP%20Third%20Person%20Character)) "MOVE_None" 0)
      (Utilities|Time|SetGlobalTimeDilation 0.01)
      (else
        (Variables|/Game/Blueprints/BPC_AttackSystemComponent.BPC_AttackSystemComponent_C|SetcanAttack? _bpc_attack_system_component true)
        (Variables|Default|SetisPanelOpened false)
        (bind _equipmentwidget (Variables|Default|GetEquipmentWidget)
          (:then
            (Widget|RemovefromParent _equipmentwidget)
            (Variables|Default|SetEquipmentWidget 0)
            (Variables|/Script/Engine.PlayerController|SetbShowMouseCursor _returnvalue false)
            (Input|SetInputModeGameOnly _returnvalue)
            (Pawn|Components|CharacterMovement|SetMovementMode (Variables|/Script/Engine.Character|GetCharacterMovement (Variables|Default|GetAs%20BP%20Third%20Person%20Character)) "MOVE_Walking" 0)
            (Utilities|Time|SetGlobalTimeDilation 1.0))
          (:else))))))

(event Input|ActionEvents|InputActionInteract
  (params (Key :type Key%20Structure))
  ;[1 1 1] Pick up Trace(old)
)

(event Input|KeyboardEvents|H
  (params (Key :type Key%20Structure))
  ;[1 1 1] Debug Show Inventory
  (:Pressed
    (for _array_element (Variables|Default|GetWeaponSlots)
      (Development|PrintString (Utilities|String|ToString(Name) (.rowname (.item _array_element)))))))

(fn AddWeapon
  (params (NewItem :type S%20Slots%20Structure%20%28by%20ref%29))
  (bind _item (Utilities|Struct|BreakS_Slots NewItem))
  (bind _as_bp_third_person_character (Variables|Default|GetAs%20BP%20Third%20Person%20Character))
  (Utilities|Array|Add (Variables|Default|GetWeaponSlots) NewItem)
  (bind _returnvalue (Utilities|GetDataTableRow (.datatable _item) (.rowname _item))
    (:then
      (switch Utilities|FlowControl|Switch|SwitchonE_WeaponTypes (.Type (Utilities|Struct|BreakS_Weapons _returnvalue))
        (:NewEnumerator0
          (Variables|/Game/ThirdPerson/Blueprints/BP_ThirdPersonCharacter.BP_ThirdPersonCharacter_C|GetEquippedItemIcon _as_bp_third_person_character
            (:then)
            (:else
              (Default|EquipMeleeItem _as_bp_third_person_character NewItem))))
        (:NewEnumerator1
          (Variables|/Game/ThirdPerson/Blueprints/BP_ThirdPersonCharacter.BP_ThirdPersonCharacter_C|GetEquippedBowIcon _as_bp_third_person_character
            (:then)
            (:else
              (Default|EquipBow _as_bp_third_person_character NewItem))))
        (:NewEnumerator3
          (Variables|/Game/ThirdPerson/Blueprints/BP_ThirdPersonCharacter.BP_ThirdPersonCharacter_C|GetEquippedShieldIcon _as_bp_third_person_character
            (:then)
            (:else
              (Default|EquipShield _as_bp_third_person_character NewItem))))
        (:NewEnumerator4
          (Variables|/Game/ThirdPerson/Blueprints/BP_ThirdPersonCharacter.BP_ThirdPersonCharacter_C|GetEquippedHealIcon _as_bp_third_person_character
            (:then)
            (:else
              (Default|EquipHeal _as_bp_third_person_character NewItem))))))))

(fn RemoveWeapon
  (params (ItemToRemove :type S%20Slots%20Structure))
  (bind _weaponslots (Variables|Default|GetWeaponSlots))
  (Utilities|Array|RemoveIndex _weaponslots (Utilities|Array|FindItem _weaponslots ItemToRemove)))