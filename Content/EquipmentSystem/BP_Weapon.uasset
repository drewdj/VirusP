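; BP_Weapon is a world weapon pickup that reads its item definition from a data table row referenced by its ItemData.
; The construction script sets the static mesh from that row.
; Its sphere overlap registers it as the PickupItem on the third-person character's equipment component and shows the item name as pickup text.
; Leaving the sphere clears the reference and hides the text.
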(event OnComponentBeginOverlap(Sphere)
  (params (OverlappedComponent :type Primitive%20Component%20Object%20Reference) (OtherActor :type Actor%20Object%20Reference) (OtherComp :type Primitive%20Component%20Object%20Reference) (OtherBodyIndex :type Integer) (bFromSweep :type Boolean) (SweepResult :type Hit%20Result%20Structure%20%28by%20ref%29))
  (bind _itemdata (Variables|Default|GetItemData))
  (bind _item (Utilities|Struct|BreakS_Slots _itemdata))
  (bind _asbp_third_person_character (Utilities|Casting|CastToBP_ThirdPersonCharacter OtherActor))
  (Variables|/Game/EquipmentSystem/BPC_EquipmentSystem.BPC_EquipmentSystem_C|SetPickupItem (Variables|/Game/ThirdPerson/Blueprints/BP_ThirdPersonCharacter.BP_ThirdPersonCharacter_C|GetBPC_EquipmentSystem _asbp_third_person_character) self)
  (bind _returnvalue (Utilities|GetDataTableRow (.datatable _item) (.rowname _item))
    (:then
      (Default|UpdatePickUpText _asbp_third_person_character (.Name (Utilities|Struct|BreakS_Weapons _returnvalue))))))

(event OnComponentEndOverlap(Sphere)
  (params (OverlappedComponent :type Primitive%20Component%20Object%20Reference) (OtherActor :type Actor%20Object%20Reference) (OtherComp :type Primitive%20Component%20Object%20Reference) (OtherBodyIndex :type Integer))
  (bind _asbp_third_person_character (Utilities|Casting|CastToBP_ThirdPersonCharacter OtherActor))
  (Variables|/Game/EquipmentSystem/BPC_EquipmentSystem.BPC_EquipmentSystem_C|SetPickupItem (Variables|/Game/ThirdPerson/Blueprints/BP_ThirdPersonCharacter.BP_ThirdPersonCharacter_C|GetBPC_EquipmentSystem _asbp_third_person_character) 0)
  (Default|DisablePickupText _asbp_third_person_character))

(fn ConstructionScript
  (bind _itemdata (Variables|Default|GetItemData))
  (bind _returnvalue (Utilities|GetDataTableRow (.datatable (.item _itemdata)) (.rowname (.item _itemdata)))
    (:then
      (Components|StaticMesh|SetStaticMesh (Variables|Default|GetStaticMesh) (.StaticMesh (Utilities|Struct|BreakS_Weapons _returnvalue))))))