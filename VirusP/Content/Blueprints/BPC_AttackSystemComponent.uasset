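; Attack component for the third-person character that runs a four-step melee combo of sword attacks and a kick.
; Attack input while armed starts a montage or buffers the next step, which SwordAttackCombo plays or resets.
; Attacks launch the character toward the targeting component's soft-locked enemy, while Tick turns it to face them.
; A timer-looped sword sweep and a one-shot sphere trace damage actors tagged Damageable.
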(event Custom|SwordAttack
  ;[0.06354 0.06354 0.06354] ComboSystem
  ;;[0.06354 0.06354 0.06354] SwordAttack
  (if (Variables|Default|GetisAttacking?)
    (Variables|Default|SetsaveAttack true)
    (else
      (Variables|Default|SetisAttacking? true)
      (CallFunction|Dash)
      (switch int (Variables|Default|GetattackIndex)
        (:0
          (CallFunction|Attack1))
        (:1
          (CallFunction|Attack2))
        (:2
          (CallFunction|Attack3))
        (:3
          (CallFunction|Attack4))))))

(event Custom|SwordAttackCombo
  ;[0.06354 0.06354 0.06354] ComboSystem
  ;;[0.06354 0.06354 0.06354] ComboContinue
  (if (Variables|Default|GetsaveAttack)
    (Variables|Default|SetsaveAttack false)
    (switch int (Variables|Default|GetattackIndex)
      (:0
        (CallFunction|Attack1))
      (:1
        (CallFunction|Attack2))
      (:2
        (CallFunction|Attack3))
      (:3
        (CallFunction|Attack4)))
    (else
      (CallFunction|StopCombo))))

(event Custom|StartSwordTrace
  ;[0.06354 0.06354 0.06354] Sword Trace
  (bind _returnvalue (Utilities|Time|SetTimerbyEvent (delegate Custom|SwordTraceLoop) 0.001 true))
  (Variables|Default|SetSword%20Trace%20Loop _returnvalue))

(event Custom|SwordTraceLoop
  (bind _characterbp (Variables|Default|GetCharacterBP))
  ;[0.06354 0.06354 0.06354] Sword Trace
  (bind (_outhit _returnvalue) (Collision|SphereTraceByChannel (Transformation|GetWorldLocation (Variables|/Game/ThirdPerson/Blueprints/BP_ThirdPersonCharacter.BP_ThirdPersonCharacter_C|GetSwordTopPoint _characterbp)) (Transformation|GetWorldLocation (Variables|/Game/ThirdPerson/Blueprints/BP_ThirdPersonCharacter.BP_ThirdPersonCharacter_C|GetSwordBottomPoint _characterbp)) 12.0 "TraceTypeQuery1" false 0 "ForDuration" true "(R=1.000000,G=0.000000,B=0.000000,A=1.000000)" "(R=0.000000,G=1.000000,B=0.000000,A=1.000000)" 0.5))
  (if _returnvalue
    (if (Actor|ActorHasTag (.HitActor (Collision|BreakHitResult _outhit)) "Damageable")
      (Utilities|FlowControl|DoOnce false :!label _label
        (:Completed
          (Game|Damage|ApplyDamage (.HitActor (Collision|BreakHitResult _outhit)) (Variables|/Game/ThirdPerson/Blueprints/BP_ThirdPersonCharacter.BP_ThirdPersonCharacter_C|GetTempDamage (Variables|Default|GetCharacterBP)) 0 0)
          (Utilities|FlowControl|Delay 0.01)
          (goto _label Reset))))))

(event Custom|StopSwordTrace
  ;[0.06354 0.06354 0.06354] Sword Trace
  (Utilities|Time|ClearandInvalidateTimerbyHandle (Variables|Default|GetSword%20Trace%20Loop)))

(event Custom|StopCombo
  ;[0.06354 0.06354 0.06354] ComboSystem
  ;;[0.06354 0.06354 0.06354] StopCombo/Attack
  (Variables|Default|SetisAttacking? false)
  (Variables|Default|SetattackIndex 0))

(event Custom|Attack4
  ;[0.06354 0.06354 0.06354] ComboSystem
  ;;[0.06354 0.06354 0.06354] Attack4
  (Utilities|FlowControl|DoOnce false :!label _label
    (:Completed
      (Utilities|FlowControl|Delay 0.1)
      (Animation|Montage|PlayMontage (Variables|Default|GetcharacterMesh) "/Game/Characters/VirusP_Character/Animations/OneHandedSword/Attack3_Montage.Attack3_Montage"
        (:then
          (Variables|Default|SetattackIndex 4)
          (goto _label Reset))))))

(event Custom|Attack%201
  ;[0.06354 0.06354 0.06354] ComboSystem
  ;;[0.06354 0.06354 0.06354] Attack1
  (Utilities|FlowControl|DoOnce false :!label _label
    (:Completed
      (Utilities|FlowControl|Delay 0.1)
      (Animation|Montage|PlayMontage (Variables|Default|GetcharacterMesh) "/Game/Characters/VirusP_Character/Animations/OneHandedSword/Attack1_Montage.Attack1_Montage"
        (:then
          (Variables|Default|SetattackIndex 1)
          (goto _label Reset))))))

(event Custom|Sphere%20Trace
  (bind _characterbp (Variables|Default|GetCharacterBP))
  (bind _sphere_trace (Variables|/Game/ThirdPerson/Blueprints/BP_ThirdPersonCharacter.BP_ThirdPersonCharacter_C|GetSphere%20Trace _characterbp))
  (bind _returnvalue (Transformation|GetWorldLocation _sphere_trace))
  ;[0.06354 0.06354 0.06354] Sphere Trace(stab and kick)
  (bind (_outhit _returnvalue_2) (Collision|SphereTraceByChannel _returnvalue _returnvalue 25.0 "TraceTypeQuery1" false 0 "ForDuration"))
  (if _returnvalue_2
    (if (Actor|ActorHasTag (.HitActor (Collision|BreakHitResult _outhit)) "Damageable")
      (Game|Damage|ApplyDamage (.HitActor (Collision|BreakHitResult _outhit)) (Variables|/Game/ThirdPerson/Blueprints/BP_ThirdPersonCharacter.BP_ThirdPersonCharacter_C|GetTempDamage (Variables|Default|GetCharacterBP)) 0 0))))

(event Custom|Attack2
  ;[0.06354 0.06354 0.06354] ComboSystem
  ;;[0.06354 0.06354 0.06354] Attack3
  (Utilities|FlowControl|DoOnce false :!label _label
    (:Completed
      (Utilities|FlowControl|Delay 0.1)
      (Animation|Montage|PlayMontage (Variables|Default|GetcharacterMesh) "/Game/Characters/VirusP_Character/Animations/OneHandedSword/Attack2_Montage.Attack2_Montage"
        (:then
          (Variables|Default|SetattackIndex 2)
          (goto _label Reset))))))

(event Custom|Attack3
  ;[0.06354 0.06354 0.06354] ComboSystem
  ;;[0.06354 0.06354 0.06354] Attack3
  (Utilities|FlowControl|DoOnce false :!label _label
    (:Completed
      (Utilities|FlowControl|Delay 0.1)
      (Animation|Montage|PlayMontage (Variables|Default|GetcharacterMesh) "/Game/Characters/VirusP_Character/Animations/OneHandedSword/Kick_Montage.Kick_Montage"
        (:then
          (Variables|Default|SetattackIndex 3)
          (goto _label Reset))))))

(event EventTick
  (params (DeltaSeconds :type Float%20%28single-precision%29))
  (bind _characterbp (Variables|Default|GetCharacterBP))
  (if (Variables|Default|GetisAttacking?)
    (bind _softlockedenemy (Variables|/Game/Blueprints/BPC_TargetingSystemComponent.BPC_TargetingSystemComponent_C|GetSoftLockedEnemy (Variables|/Game/ThirdPerson/Blueprints/BP_ThirdPersonCharacter.BP_ThirdPersonCharacter_C|GetBPC_TargetingSystemComponent _characterbp))
      (:then
        (Transformation|SetActorRotation _characterbp (Math|Interpolation|RInterpTo (Transformation|GetActorRotation _characterbp) (Math|Rotator|FindLookatRotation (Transformation|GetActorLocation _characterbp) (Transformation|GetActorLocation _softlockedenemy)) DeltaSeconds 1e+01)))
      (:else))))

(event EventBeginPlay
  (bind _asbp_third_person_character (Utilities|Casting|CastToBP_ThirdPersonCharacter (Components|GetOwner)))
  (Variables|Default|SetCharacterBP _asbp_third_person_character)
  (Variables|Default|SetcharacterMesh (Variables|/Script/Engine.Character|GetMesh _asbp_third_person_character)))

(event Input|ActionEvents|InputActionAttack
  (params (Key :type Key%20Structure :default "None"))
  ;[0.06354 0.06354 0.06354] ComboSystem
  ;;[0.06354 0.06354 0.06354] AttackInput
  (:Pressed
    (if (Variables|Default|GetArmed?)
      (if (Variables|Default|GetcanAttack?)
        (CallFunction|SwordAttack)))))

(fn Dash
  (bind _characterbp (Variables|Default|GetCharacterBP))
  (bind _softlockedenemy (Variables|/Game/Blueprints/BPC_TargetingSystemComponent.BPC_TargetingSystemComponent_C|GetSoftLockedEnemy (Variables|/Game/ThirdPerson/Blueprints/BP_ThirdPersonCharacter.BP_ThirdPersonCharacter_C|GetBPC_TargetingSystemComponent _characterbp))
    (:then
      (if (> (Transformation|GetDistanceTo _characterbp _softlockedenemy) 1.0)
        (Character|LaunchCharacter _characterbp (* (Math|Vector|GetForwardVector (Math|Rotator|FindLookatRotation (Transformation|GetActorLocation _characterbp) (Transformation|GetActorLocation _softlockedenemy))) 1e+03) true true)))
    (:else)))