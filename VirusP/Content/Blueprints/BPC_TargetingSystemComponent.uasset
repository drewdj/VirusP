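; Targeting component for BP_ThirdPersonCharacter that soft-locks onto a nearby BP_AI enemy.
; On BeginPlay it takes the owner's SphereComponent as the detection volume.
; Each Tick with enemies overlapping, it seeks the closest living one by distance and moves the soft-lock icon to it.
; The lock clears if the selected enemy is dead or beyond the sphere radius, checked only while enemies overlap.
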(event EventBeginPlay
  ;[1 1 1] BeginPlay
  ;;[1 1 1] Set SoftLock Sphere
  (bind _asbp_third_person_character (Utilities|Casting|CastToBP_ThirdPersonCharacter (Components|GetOwner)))
  (Variables|Default|SetSoftLockSphere (Actor|GetComponentbyClass _asbp_third_person_character "/Script/Engine.SphereComponent")))

(event EventTick
  (params (DeltaSeconds :type Float%20%28single-precision%29))
  (bind _softlocksphere (Variables|Default|GetSoftLockSphere))
  (bind _overlappingactors (Collision|GetOverlappingActors _softlocksphere "/Game/AI/BP_AI.BP_AI_C" :!class /Script/Engine.PrimitiveComponent))
  (bind _output (Utilities|Array|Get(acopy) _overlappingactors))
  ;[1 1 1] Check enemies in sphere
  (if (> (Utilities|Array|Length _overlappingactors) 0)
    ;[1 1 1] Set SoftlockedActor and Mindistance
    (bind _asbp_ai (Utilities|Casting|CastToBP_AI _output))
    (Variables|Default|SetSoftLockedEnemy _asbp_ai)
    (Variables|Default|SetMinDistance (Transformation|GetDistanceTo _output (Components|GetOwner)))
    (for _array_element _overlappingactors
      (bind _asbp_ai_2 (Utilities|Casting|CastToBP_AI _array_element))
      (Default|DisableSoftlockIcon _asbp_ai_2)
      ;[1 1 1] Enemy Dead?
      (if (not (Variables|/Script/VirusP.HealthComponent|GetbIsDead (Variables|/Game/AI/BP_AI.BP_AI_C|GetHealth _asbp_ai_2)))
        ;[1 1 1] Closer to new enemy?
        (if (<= (Transformation|GetDistanceTo _array_element (Components|GetOwner)) (Variables|Default|GetMinDistance))
          (Variables|Default|SetSoftLockedEnemy _asbp_ai_2)
          (Variables|Default|SetMinDistance (Transformation|GetDistanceTo _array_element (Components|GetOwner))))))
    (Default|EnableSoftlockIcon (Variables|Default|GetSoftLockedEnemy))
    ;[1 1 1] If enemyFar disable softlock
    (if (> (Transformation|GetDistanceTo (Variables|Default|GetSoftLockedEnemy) (Components|GetOwner)) (Variables|/Script/Engine.SphereComponent|GetSphereRadius (Variables|Default|GetSoftLockSphere)))
      (Default|DisableSoftlockIcon (Variables|Default|GetSoftLockedEnemy))
      (Variables|Default|SetSoftLockedEnemy 0)
      (else
        ;[1 1 1] If enemyDead disable
        (if (Variables|/Script/VirusP.HealthComponent|GetbIsDead (Variables|/Game/AI/BP_AI.BP_AI_C|GetHealth (Variables|Default|GetSoftLockedEnemy)))
          (Default|DisableSoftlockIcon (Variables|Default|GetSoftLockedEnemy))
          (Variables|Default|SetSoftLockedEnemy 0))))))