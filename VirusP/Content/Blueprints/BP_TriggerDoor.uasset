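; BP_TriggerDoor is a door that swings open when the third-person character walks into one of its two trigger boxes.
; Each box's overlap event plays its own timeline, which scales that box's angle variable to set the door's relative yaw.
; A shared Open flag lets only the first trigger act, and nothing in the graph closes the door again.
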(event OnComponentBeginOverlap(Box)
  (params (OverlappedComponent :type Primitive%20Component%20Object%20Reference) (OtherActor :type Actor%20Object%20Reference) (OtherComp :type Primitive%20Component%20Object%20Reference) (OtherBodyIndex :type Integer) (bFromSweep :type Boolean) (SweepResult :type Hit%20Result%20Structure%20%28by%20ref%29))
  (if (not (Variables|Default|GetOpen))
    (Utilities|Casting|CastToBP_ThirdPersonCharacter OtherActor)
    (Variables|Default|SetOpen true)
    (bind _newtrack_0 (Timeline|Timeline_0 Play)
      (:Update
        (Transformation|SetRelativeRotation (Variables|Default|GetDoor) (Math|Rotator|MakeRotator 0.0 0.0 (* _newtrack_0 (Variables|Default|GetAngle_1))) false false)))))

(event OnComponentBeginOverlap(Box1)
  (params (OverlappedComponent :type Primitive%20Component%20Object%20Reference) (OtherActor :type Actor%20Object%20Reference) (OtherComp :type Primitive%20Component%20Object%20Reference) (OtherBodyIndex :type Integer) (bFromSweep :type Boolean) (SweepResult :type Hit%20Result%20Structure%20%28by%20ref%29))
  (if (not (Variables|Default|GetOpen))
    (Utilities|Casting|CastToBP_ThirdPersonCharacter OtherActor)
    (Variables|Default|SetOpen true)
    (bind _newtrack_0 (Timeline|Timeline_1 Play)
      (:Update
        (Transformation|SetRelativeRotation (Variables|Default|GetDoor) (Math|Rotator|MakeRotator 0.0 0.0 (* _newtrack_0 (Variables|Default|GetAngle_2))) false false)))))

(fn ConstructionScript)