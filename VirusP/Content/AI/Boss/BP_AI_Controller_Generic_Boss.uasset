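; AI controller for a generic boss that runs its behavior tree and manages combat presentation.
; ActivateBossCombat creates the health bar widget and, through a DoOnce, pauses the player's base music, plays a growl, then starts boss music after a delay and stores it on the boss pawn.
; Tick updates the bar from the boss's health ratio.
; DeactivateBossCombat only removes the bar, leaving music untouched.
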(event Custom|DeactivateBossCombat
  (bind _bosshealthbarwidget (Variables|Default|GetBossHealthBarWidget)
    (:then
      (Widget|RemovefromParent _bosshealthbarwidget)
      (Variables|Default|SetBossHealthBarWidget 0))
    (:else)))

(event Custom|ActivateBossCombat
  (bind _returnvalue (UserInterface|CreateWidget "/Game/Blueprints/Widgets/WBP_BossHealthBar.WBP_BossHealthBar_C"))
  (bind _output_get (Variables|Default|SetBossHealthBarWidget _returnvalue))
  (UserInterface|Viewport|AddtoViewport _output_get 0)
  (Utilities|FlowControl|DoOnce false
    (:Completed
      (bind _asbp_third_person_character (Utilities|Casting|CastToBP_ThirdPersonCharacter (Game|GetPlayerCharacter 0)))
      (Class|AudioComponent|SetPaused (Variables|/Game/ThirdPerson/Blueprints/BP_ThirdPersonCharacter.BP_ThirdPersonCharacter_C|GetBaseMusic _asbp_third_person_character) true)
      (Audio|PlaySoundatLocation "/Game/Audio/enemy/boss_grawl_Cue.boss_grawl_Cue" (Transformation|GetActorLocation (Pawn|GetControlledPawn)) "0, 0, 0" 1.0 1.0 0.0 0 0 0 0)
      (Utilities|FlowControl|Delay 2.0)
      (bind _returnvalue_2 (Audio|SpawnSound2D "/Game/Audio/music_1_Cue.music_1_Cue" 1.0 1.0 0.0 0))
      (Components|Activation|SetActive _returnvalue_2 true false)
      (Variables|/Game/AI/Boss/BP_AI_Boss.BP_AI_Boss_C|SetBossMusic (Variables|Default|GetBP%20AI%20Boss) _returnvalue_2))))

(event EventBeginPlay
  (AI|RunBehaviorTree "/Game/AI/Boss/BT_AI_Boss.BT_AI_Boss")
  (bind _asbp_ai_boss (Utilities|Casting|CastToBP_AI_Boss (Pawn|GetControlledPawn)))
  (Variables|Default|SetBP%20AI%20Boss _asbp_ai_boss))

(event EventTick
  (params (DeltaSeconds :type Float%20%28single-precision%29))
  (bind _bp_ai_boss (Variables|Default|GetBP%20AI%20Boss))
  (bind _health (Variables|/Game/AI/BP_AI.BP_AI_C|GetHealth _bp_ai_boss))
  (bind _bosshealthbarwidget (Variables|Default|GetBossHealthBarWidget)
    (:then
      (Progress|SetPercent (Variables|/Game/Blueprints/Widgets/WBP_BossHealthBar.WBP_BossHealthBar_C|GetProgressHealthBar _bosshealthbarwidget) (/ (Variables|/Script/VirusP.HealthComponent|GetHealth _health) (Variables|/Script/VirusP.HealthComponent|GetDefaultHealth _health))))
    (:else)))

(fn ConstructionScript
  (|CallParentFunction))