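; BP_AI_Boss is a boss AI character that sets its experience value to 500 on begin play and handles the end of its fight.
; On Health death, it tells its generic boss AI controller to deactivate boss combat, stops the boss music and plays a damage sound at its location.
; After a short delay, it resumes the player's paused base music.
; Tick and construction only call the parent.
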(event OnDeath(Health)
  (bind _asbp_ai_controller_generic_boss (Utilities|Casting|CastToBP_AI_Controller_Generic_Boss (Pawn|GetController)))
  (Default|DeactivateBossCombat _asbp_ai_controller_generic_boss)
  (Audio|Components|Audio|Stop (Variables|Default|GetBossMusic))
  (Audio|PlaySoundatLocation "/Game/Audio/enemy/damage_Cue.damage_Cue" (Transformation|GetActorLocation) "0, 0, 0" 1.0 0.3 0.0 0 0 0 0)
  (Utilities|FlowControl|Delay 2.0)
  (Class|AudioComponent|SetPaused (Variables|/Game/ThirdPerson/Blueprints/BP_ThirdPersonCharacter.BP_ThirdPersonCharacter_C|GetBaseMusic (Variables|Default|GetPlayerCharacter)) false))

(event EventBeginPlay
  (|CallParentFunction)
  (Variables|Default|SetExperience 5e+02))

(event Collision|EventActorBeginOverlap
  (params (OtherActor :type Actor%20Object%20Reference)))

(event EventTick
  (params (DeltaSeconds :type Float%20%28single-precision%29))
  (|CallParentFunction DeltaSeconds))

(fn ConstructionScript
  (|CallParentFunction))