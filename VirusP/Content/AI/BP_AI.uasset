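; Melee enemy character Blueprint that fights with sword combos, reacts to damage and grants the player XP on death.
; Behavior tree attack calls chain montages through AttackIndex and a buffered SaveAttack flag, while timer-looped or one-shot sphere traces damage "Damageable" actors.
; Tick turns health, investigate and softlock widgets toward the camera and rotates the attacker toward its target.
; A dynamic material shows red alert and a timed rage state.
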(event OnDeath(Health)
  (bind _returnvalue (Pawn|GetController))
  (Class|LevelComponent|AddExperience (Variables|/Script/VirusP.VirusPCharacter|GetLevelComponent (Variables|Default|GetPlayerCharacter)) 3e+01)
  (if (Utilities|IsValid _returnvalue)
    (Pawn|UnPossess _returnvalue)
    (Rendering|SetVisibility (Variables|Default|GetHealthBarWidget) false false)
    (Collision|SetCollisionEnabled (Variables|Collision|GetCapsuleComponent) "NoCollision")
    ;[1 1 1] Cambiar a  solo si he matado al que tengo lockeado
    (Default|DisableTargetLock (Variables|Default|GetPlayerCharacter))))

(event Custom|SwordAttack
  ;[0.06354 0.06354 0.06354] ComboSystem
  ;;[0.06354 0.06354 0.06354] SwordAttack
  (if (Variables|Default|GetisAttacking?)
    (Variables|Default|SetsaveAttack true)
    (else
      (Variables|Default|SetisAttacking? true)
      (switch int (Variables|Default|GetattackIndex)
        (:0
          (CallFunction|Attack1))
        (:1
          (CallFunction|Attack2))
        (:2
          (CallFunction|Attack4))))))

(event Custom|SwordAttackCombo
  ;[0.06354 0.06354 0.06354] ComboSystem
  ;;[0.06354 0.06354 0.06354] ComboContinue
  (if (Variables|Default|GetsaveAttack)
    (Variables|Default|SetsaveAttack false)
    (switch int (Variables|Default|GetattackIndex)
      (:0
        (CallFunction|Attack1))
      (:1
        (CallFunction|Attack2))
      (:2
        (CallFunction|Attack4)))
    (else
      (CallFunction|StopCombo))))

(event Custom|StartSwordTrace
  ;[0.06354 0.06354 0.06354] Sword Trace
  (bind _returnvalue (Utilities|Time|SetTimerbyEvent (delegate Custom|SwordTraceLoop) 0.001 true))
  (Variables|Default|SetSword%20Trace%20Loop _returnvalue))

(event Custom|SwordTraceLoop
  ;[0.06354 0.06354 0.06354] Sword Trace
  (bind (_outhit _returnvalue) (Collision|SphereTraceByChannel (Transformation|GetWorldLocation (Variables|Default|GetSwordTopPoint)) (Transformation|GetWorldLocation (Variables|Default|GetSwordBottomPoint)) 12.0 "TraceTypeQuery1" false 0 "ForDuration" true "(R=1.000000,G=0.000000,B=0.000000,A=1.000000)" "(R=0.000000,G=1.000000,B=0.000000,A=1.000000)" 0.5))
  (if _returnvalue
    (if (Actor|ActorHasTag (.HitActor (Collision|BreakHitResult _outhit)) "Damageable")
      (Utilities|FlowControl|DoOnce false :!label _label
        (:Completed
          (Game|Damage|ApplyDamage (.HitActor (Collision|BreakHitResult _outhit)) (Variables|Default|GetBase%20Damage) 0 0)
          (Utilities|FlowControl|Delay 0.5)
          (goto _label Reset))))))

(event Custom|StopSwordTrace
  ;[0.06354 0.06354 0.06354] Sword Trace
  (Utilities|Time|ClearandInvalidateTimerbyHandle (Variables|Default|GetSword%20Trace%20Loop)))

(event Custom|EnableSoftlockIcon
  (Rendering|SetVisibility (Variables|Default|GetSoftlockWidget) true false))

(event Custom|Sword%20Attack%20Combo%20Call%20From%20BT
  ;[0.06354 0.06354 0.06354] ComboSystem
  ;;[0.06354 0.06354 0.06354] AttackInput
  (if (Variables|Default|GetcanAttack?)
    (CallFunction|SwordAttack)))

(event Custom|SetEnemy
  (Variables|Default|SetEnemy true)
  (CallFunction|Rageon)
  (Utilities|FlowControl|Delay 15.0)
  (Variables|Default|SetEnemy false)
  (CallFunction|RageOff))

(event Custom|RedAlertOn
  (bind _mesh (Variables|Character|GetMesh))
  (bind _enemymaterial (Variables|Default|GetEnemyMaterial))
  (Rendering|Material|SetScalarParameterValue _enemymaterial "RedAlert" 1.0 :!class /Script/Engine.MaterialInstanceDynamic)
  (Rendering|Material|SetMaterial _mesh 0 _enemymaterial)
  (Rendering|Material|SetMaterial _mesh 1 _enemymaterial)
  (Development|PrintString "RedAler"))

(event Custom|RageOff
  (bind _mesh (Variables|Character|GetMesh))
  (bind _enemymaterial (Variables|Default|GetEnemyMaterial))
  (Rendering|Material|SetScalarParameterValue _enemymaterial "Rage" 0.0 :!class /Script/Engine.MaterialInstanceDynamic)
  (Rendering|Material|SetMaterial _mesh 0 _enemymaterial)
  (Rendering|Material|SetMaterial _mesh 1 _enemymaterial))

(event Custom|RedAlertOff
  (bind _mesh (Variables|Character|GetMesh))
  (bind _enemymaterial (Variables|Default|GetEnemyMaterial))
  (Rendering|Material|SetScalarParameterValue _enemymaterial "RedAlert" 0.0 :!class /Script/Engine.MaterialInstanceDynamic)
  (Rendering|Material|SetMaterial _mesh 0 _enemymaterial)
  (Rendering|Material|SetMaterial _mesh 1 _enemymaterial))

(event Custom|StopCombo
  ;[0.06354 0.06354 0.06354] ComboSystem
  ;;[0.06354 0.06354 0.06354] StopCombo/Attack
  (Variables|Default|SetisAttacking? false)
  (Variables|Default|SetattackIndex 0))

(event Custom|RageOn
  (bind _mesh (Variables|Character|GetMesh))
  (bind _enemymaterial (Variables|Default|GetEnemyMaterial))
  (Rendering|Material|SetScalarParameterValue _enemymaterial "Rage" 1.0 :!class /Script/Engine.MaterialInstanceDynamic)
  (Rendering|Material|SetMaterial _mesh 0 _enemymaterial)
  (Rendering|Material|SetMaterial _mesh 1 _enemymaterial)
  (Development|PrintString "Rage"))

(event Custom|Attack4
  ;[0.06354 0.06354 0.06354] ComboSystem
  ;;[0.06354 0.06354 0.06354] Attack4
  (Utilities|FlowControl|DoOnce false :!label _label
    (:Completed
      (Utilities|FlowControl|Delay 0.1)
      (Animation|Montage|PlayMontage (Variables|Character|GetMesh) "/Game/Characters/VirusP_Character/Animations/OneHandedSword/Attack3_Montage.Attack3_Montage" (Variables|Default|GetAttackAnimationSpeed)
        (:then
          (Variables|Default|SetattackIndex 4)
          (goto _label Reset))))))

(event Custom|Attack%201
  ;[0.06354 0.06354 0.06354] ComboSystem
  ;;[0.06354 0.06354 0.06354] Attack1
  (Utilities|FlowControl|DoOnce false :!label _label
    (:Completed
      (Utilities|FlowControl|Delay 0.1)
      (Animation|Montage|PlayMontage (Variables|Character|GetMesh) "/Game/Characters/VirusP_Character/Animations/OneHandedSword/Attack1Short_Montage.Attack1Short_Montage" (Variables|Default|GetAttackAnimationSpeed)
        (:then
          (Variables|Default|SetattackIndex 1)
          (goto _label Reset))))))

(event Custom|Sphere%20Trace
  (bind _sphere_trace1 (Variables|Default|GetSphere%20Trace1))
  (bind _returnvalue (Transformation|GetWorldLocation _sphere_trace1))
  ;[0.06354 0.06354 0.06354] Sphere Trace(stab and kick)
  (bind (_outhit _returnvalue_2) (Collision|SphereTraceByChannel _returnvalue _returnvalue 25.0 "TraceTypeQuery1" false 0 "ForDuration"))
  (if _returnvalue_2
    (if (Actor|ActorHasTag (.HitActor (Collision|BreakHitResult _outhit)) "Damageable")
      (Game|Damage|ApplyDamage (.HitActor (Collision|BreakHitResult _outhit)) (Variables|Default|GetBase%20Damage) 0 0))))

(event Custom|Attack2
  ;[0.06354 0.06354 0.06354] ComboSystem
  ;;[0.06354 0.06354 0.06354] Attack3
  (Utilities|FlowControl|DoOnce false :!label _label
    (:Completed
      (Utilities|FlowControl|Delay 0.1)
      (Animation|Montage|PlayMontage (Variables|Character|GetMesh) "/Game/Characters/VirusP_Character/Animations/OneHandedSword/Attack2_Montage.Attack2_Montage" (Variables|Default|GetAttackAnimationSpeed)
        (:then
          (Variables|Default|SetattackIndex 2)
          (goto _label Reset))))))

(event Custom|Toggle%20Investigation%20Icon
  (bind _investigatewidget (Variables|Default|GetInvestigateWidget))
  (Utilities|FlowControl|FlipFlop
    (:A
      (Rendering|SetVisibility _investigatewidget true false))
    (:B
      (Rendering|SetVisibility _investigatewidget false false))))

(event Custom|Attack3
  ;[0.06354 0.06354 0.06354] ComboSystem
  ;;[0.06354 0.06354 0.06354] Attack3
  (Utilities|FlowControl|DoOnce false :!label _label
    (:Completed
      (Utilities|FlowControl|Delay 0.1)
      (Animation|Montage|PlayMontage (Variables|Character|GetMesh) "/Game/Characters/VirusP_Character/Animations/OneHandedSword/Kick_Montage.Kick_Montage" (Variables|Default|GetAttackAnimationSpeed)
        (:then
          (Variables|Default|SetattackIndex 3)
          (goto _label Reset))))))

(event Custom|DisableSoftlockIcon
  (Rendering|SetVisibility (Variables|Default|GetSoftlockWidget) false false))

(event EventBeginPlay
  (bind _asbp_third_person_character (Utilities|Casting|CastToBP_ThirdPersonCharacter (Game|GetPlayerCharacter 0)))
  (Variables|Default|SetPlayerCharacter _asbp_third_person_character)
  (bind _returnvalue (Rendering|Material|CreateDynamicMaterialInstance "/Game/Materials/Enemy.Enemy" "None" "None" :!class /Script/Engine.KismetMaterialLibrary))
  (Variables|Default|SetEnemyMaterial _returnvalue))

(event Game|Damage|EventAnyDamage
  (params (Damage :type Float%20%28single-precision%29) (DamageType :type Damage%20Type%20Object%20Reference) (InstigatedBy :type Controller%20Object%20Reference) (DamageCauser :type Actor%20Object%20Reference))
  (Animation|PlayAnimMontage (Utilities|Array|Get(acopy) (Variables|Default|GetHitAnims) (Math|Random|RandomIntegerinRange 0 (- (Utilities|Array|Length (Variables|Default|GetHitAnims)) 1))) 1.0 "None")
  (CallFunction|StopCombo))

(event EventTick
  (params (DeltaSeconds :type Float%20%28single-precision%29))
  (bind _healthbarwidget (Variables|Default|GetHealthBarWidget))
  (bind _health (Variables|Default|GetHealth))
  (bind _aswbp_health_bar (Utilities|Casting|CastToWBP_HealthBar (UserInterface|GetWidget (Variables|Default|GetHealthBarWidget))))
  (Progress|SetPercent (Variables|/Game/Blueprints/Widgets/WBP_HealthBar.WBP_HealthBar_C|GetHealthBar _aswbp_health_bar) (/ (Variables|/Script/VirusP.HealthComponent|GetHealth _health) (Variables|/Script/VirusP.HealthComponent|GetDefaultHealth _health)))
  (Transformation|SetWorldRotation _healthbarwidget (Math|Rotator|FindLookatRotation (Transformation|GetWorldLocation _healthbarwidget) (Transformation|GetWorldLocation (Variables|/Script/Engine.PlayerCameraManager|GetTransformComponent (Game|GetPlayerCameraManager 0)))) false false)
  (bind _tohit (Variables|Default|GetToHit)
    (:then
      (if (Variables|Default|GetisAttacking?)
        (Transformation|SetActorRotation (Math|Interpolation|RInterpTo (Transformation|GetActorRotation) (Math|Rotator|FindLookatRotation (Transformation|GetActorLocation) (Transformation|GetActorLocation _tohit)) DeltaSeconds 1e+01))))
    (:else)))

(fn ConstructionScript)

(fn Attack
  (CallFunction|SwordAttackComboCallfromBT)
  (return 0.4))