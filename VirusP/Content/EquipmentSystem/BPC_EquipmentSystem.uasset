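; Equipment component for the third-person character that handles weapon pickup and the equipment menu.
; Interact sphere-traces from the follow camera, stores a hit BP_Weapon's item data in the WeaponSlots array and destroys the actor.
; The EquipmentMenu input toggles the WBP_Equipment widget, switching cursor and input mode and blocking movement and attacks while open.
; A debug key prints the stored weapons' row names.
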(event EventBeginPlay
  ;[1 1 1] Set variables
  (bind _asbp_third_person_character (Utilities|Casting|CastToBP_ThirdPersonCharacter (Components|GetOwner)))
  (Variables|Default|SetFollow%20Camera (Variables|/Script/VirusP.VirusPCharacter|GetFollowCamera _asbp_third_person_character))
  (Variables|Default|SetBPC%20Attack%20System%20Component (Variables|/Game/ThirdPerson/Blueprints/BP_ThirdPersonCharacter.BP_ThirdPersonCharacter_C|GetBPC_AttackSystemComponent _asbp_third_person_character)))

(event Input|ActionEvents|InputActionInteract
  (params (Key :type Key%20Structure :default "None"))
  (bind _follow_camera (Variables|Default|GetFollow%20Camera))
  (bind _returnvalue (Transformation|GetWorldLocation _follow_camera))
  ;[1 1 1] Pick up Trace
  (:Pressed
    (bind (_outhit _returnvalue_2) (Collision|SphereTraceForObjects _returnvalue (+ _returnvalue (* (Math|Vector|GetForwardVector (Transformation|GetWorldRotation _follow_camera)) 1e+03)) 15.0 (Utilities|Array|MakeArray "ObjectTypeQuery2") false 0 "ForDuration"))
    (if _returnvalue_2
      (bind _asbp_weapon (Utilities|Casting|CastToBP_Weapon (.HitActor (Collision|BreakHitResult _outhit))))
      (CallFunction|AddWeapon (Variables|/Game/EquipmentSystem/BP_Weapon.BP_Weapon_C|GetItemData _asbp_weapon))
      (Actor|DestroyActor _asbp_weapon))))

(event Input|ActionEvents|InputActionEquipmentMenu
  (params (Key :type Key%20Structure :default "None"))
  (bind _returnvalue (Game|GetPlayerController 0))
  (bind _returnvalue_2 (Components|GetOwner))
  (bind _bpc_attack_system_component (Variables|Default|GetBPC%20Attack%20System%20Component))
  ;[1 1 1] Equipment menu panel
  (:Pressed
    (if (not (Variables|Default|GetisPanelOpened))
      (Variables|/Game/Blueprints/BPC_AttackSystemComponent.BPC_AttackSystemComponent_C|SetcanAttack? _bpc_attack_system_component false)
      (Variables|Default|SetisPanelOpened true)
      (bind _returnvalue_3 (UserInterface|CreateWidget "/Game/Blueprints/Widgets/WBP_Equipment.WBP_Equipment_C"))
      (bind _output_get (Variables|Default|SetEquipmentWidget _returnvalue_3))
      (UserInterface|Viewport|AddtoViewport _output_get 0)
      (Variables|/Script/Engine.PlayerController|SetbShowMouseCursor _returnvalue true)
      (Input|SetInputModeGameandUI _returnvalue (Variables|Default|GetEquipmentWidget) "DoNotLock" true)
      (bind _asbp_third_person_character (Utilities|Casting|CastToBP_ThirdPersonCharacter _returnvalue_2))
      (Pawn|Components|CharacterMovement|SetMovementMode (Variables|/Script/Engine.Character|GetCharacterMovement _asbp_third_person_character) "MOVE_None" 0)
      (else
        (Variables|/Game/Blueprints/BPC_AttackSystemComponent.BPC_AttackSystemComponent_C|SetcanAttack? _bpc_attack_system_component true)
        (Variables|Default|SetisPanelOpened false)
        (bind _equipmentwidget (Variables|Default|GetEquipmentWidget)
          (:then
            (Widget|RemovefromParent _equipmentwidget)
            (Variables|Default|SetEquipmentWidget 0)
            (Variables|/Script/Engine.PlayerController|SetbShowMouseCursor _returnvalue false)
            (Input|SetInputModeGameOnly _returnvalue)
            (bind _asbp_third_person_character_2 (Utilities|Casting|CastToBP_ThirdPersonCharacter _returnvalue_2))
            (Pawn|Components|CharacterMovement|SetMovementMode (Variables|/Script/Engine.Character|GetCharacterMovement _asbp_third_person_character_2) "MOVE_Walking" 0))
          (:else))))))

(event Input|KeyboardEvents|H
  (params (Key :type Key%20Structure :default "None"))
  ;[1 1 1] Debug Show Inventory
  (:Pressed
    (for _array_element (Variables|Default|GetWeaponSlots)
      (Development|PrintString (Utilities|String|ToString(Name) (.rowname (.item _array_element)))))))

(fn AddWeapon
  (params (NewItem :type S%20Slots%20Structure%20%28by%20ref%29))
  (Utilities|Array|Add (Variables|Default|GetWeaponSlots) NewItem))